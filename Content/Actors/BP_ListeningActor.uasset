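; BP_ListeningActor is a replicated actor that destroys itself when a boolean it monitors on TargetActor changes.
; On BeginPlay, only with network authority, it starts a ListenForBooleanChange async task, stores the task handle and routes Value Changed to a DoOnce-guarded destroy.
; An unconnected test event prints the new value and stops listening through the stored handle after a delay.
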(event `self.ReceiveBeginPlay`
  (if (`self.HasAuthority`)
    (bind (_asynctaskproxy _newvalue) (`AsyncTask_ListenForBooleanChange.ListenForBooleanChange` (`self.TargetActor`))
      (:`then`
        (set `self.AsyncTask ListenForBooleanChange` _asynctaskproxy))
      (:`OnValueChanged`
        (`self.DestroyListeningActor`)))))

(event `DestroyListeningActor`
  (`/Engine/EditorBlueprintResources/StandardMacros.DoOnce` false ; this node is not neccessary but serves as additional safeguard
    (:`Completed`
      (`self.K2_DestroyActor`))))

(event `TestOnValueChaged`
  (params (bNewValue :type Boolean))
  ;[1 1 1] For Testing Only - OnValueChanged
  (`KismetSystemLibrary.PrintText` (`|FormatText` "Value Changed to {NewValue}" bNewValue))
  (`/Engine/EditorBlueprintResources/StandardMacros.DoOnce` false
    (:`Completed`
      (`KismetSystemLibrary.PrintString` "ListeningActor will stop listening after 10 seconds" true true (struct :`G` 1.0 :`A` 1.0) 4.0)
      (`KismetSystemLibrary.Delay` 10.0)
      (`AsyncTask_ListenForBooleanChange.StopListening` (`self.AsyncTask ListenForBooleanChange`))
      (`KismetSystemLibrary.PrintString` "ListeningActor stopped listening to boolean change" true true (struct :`G` 1.0 :`A` 1.0) 4.0))))

(fn `UserConstructionScript`)